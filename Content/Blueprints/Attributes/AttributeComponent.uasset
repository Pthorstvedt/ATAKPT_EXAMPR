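; Player attribute component on TimelessCharacter that tracks level and XP for seven RPG stats from Vitality to Charisma.
; BeginPlay loads the attribute struct from the game instance's save data, then sets full health.
; Each AddXP function levels at its threshold, discarding overflow and multiplying the next requirement by XPRequiredExponent.
; Level-ups save to slot and show a timed popup; Vitality also raises MaxHealth and rescales the HP bar.
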(event Custom|LevelUp
  (params (SkillUpText :type Text))
  (CallFunction|SaveAttributes)
  (Variables|Default|GetLvLText_WG
    (:then
      (Utilities|FlowControl|Delay 2.0))
    (:else
      _))
  (bind _returnvalue (UserInterface|CreateWidget "/Game/Blueprints/UI/LevelUpText.LevelUpText_C" (Game|GetPlayerController 0) SkillUpText))
  (bind _output_get (Variables|Default|SetLvLText_WG _returnvalue))
  (UserInterface|Viewport|AddtoViewport _output_get 0)
  (Utilities|FlowControl|Delay 2.0)
  (Widget|RemovefromParent _output_get)
  (Variables|Default|SetLvLText_WG 0))

(event Custom|SaveAttributes
  (bind _as_timeless_instance (Variables|Default|GetAs%20Timeless%20Instance))
  (bind _savegamedata (Variables|/Game/Blueprints/TimelessInstance.TimelessInstance_C|GetSaveGameData _as_timeless_instance))
  (Variables|/Game/Blueprints/SaveGameObject.SaveGameObject_C|SetPlayerAttributes_Save _savegamedata (Variables|Default|GetAttributeStruct))
  (SaveGame|SaveGametoSlot _savegamedata (Variables|/Game/Blueprints/TimelessInstance.TimelessInstance_C|GetSaveGameName _as_timeless_instance)))

(event EventBeginPlay
  ;[1 1 1] Load Attributes on BeginPlay
  (bind _astimeless_character (Utilities|Casting|CastToTimelessCharacter (Components|GetOwner)))
  (Variables|Default|SetAs%20Timeless%20Character _astimeless_character)
  (bind _astimeless_instance (Utilities|Casting|CastToTimelessInstance (Game|GetGameInstance)))
  (bind _output_get (Variables|Default|SetAs%20Timeless%20Instance _astimeless_instance))
  (Variables|Default|SetAttributeStruct (Variables|/Game/Blueprints/SaveGameObject.SaveGameObject_C|GetPlayerAttributes_Save (Variables|/Game/Blueprints/TimelessInstance.TimelessInstance_C|GetSaveGameData _output_get)))
  (Utilities|FlowControl|Delay 0.1)
  (CallFunction|SetHPValues true))

(fn AddVITxp
  (params (XPyield :type Float%20%28single-precision%29))
  (bind _output_get (Variables|Default|SetAttributeStruct (Utilities|Struct|MakeAttributeStruct (.vit_lvl (Variables|Default|GetAttributeStruct)) (+ (.vit_xp (Variables|Default|GetAttributeStruct)) XPyield) (.vit_xp_required (Variables|Default|GetAttributeStruct)) (.str_lvl (Variables|Default|GetAttributeStruct)) (.str_xp (Variables|Default|GetAttributeStruct)) (.str_xp_required (Variables|Default|GetAttributeStruct)) (.end_lvl (Variables|Default|GetAttributeStruct)) (.end_xp (Variables|Default|GetAttributeStruct)) (.end_xp_required (Variables|Default|GetAttributeStruct)) (.fin_lvl (Variables|Default|GetAttributeStruct)) (.fin_xp (Variables|Default|GetAttributeStruct)) (.fin_xp_required (Variables|Default|GetAttributeStruct)) (.int_lvl (Variables|Default|GetAttributeStruct)) (.int_xp (Variables|Default|GetAttributeStruct)) (.int_xp_required (Variables|Default|GetAttributeStruct)) (.wis_lvl (Variables|Default|GetAttributeStruct)) (.wis_xp (Variables|Default|GetAttributeStruct)) (.wis_xp_required (Variables|Default|GetAttributeStruct)) (.cha_lvl (Variables|Default|GetAttributeStruct)) (.cha_xp (Variables|Default|GetAttributeStruct)) (.cha_xp_required (Variables|Default|GetAttributeStruct)))))
  (if (>= (.vit_xp (Variables|Default|GetAttributeStruct)) (.vit_xp_required (Variables|Default|GetAttributeStruct)))
    (bind _output_get_2 (Variables|Default|SetAttributeStruct (Utilities|Struct|MakeAttributeStruct (+ (.vit_lvl _output_get) 1) 0.0 (Math|Conversions|ToFloat(Integer) (Math|Float|Round (* (.vit_xp_required _output_get) (Variables|Default|GetXP_Required_Exponent)))) (.str_lvl _output_get) (.str_xp _output_get) (.str_xp_required _output_get) (.end_lvl _output_get) (.end_xp _output_get) (.end_xp_required _output_get) (.fin_lvl _output_get) (.fin_xp _output_get) (.fin_xp_required _output_get) (.int_lvl _output_get) (.int_xp _output_get) (.int_xp_required _output_get) (.wis_lvl _output_get) (.wis_xp _output_get) (.wis_xp_required _output_get) (.cha_lvl _output_get) (.cha_xp _output_get) (.cha_xp_required _output_get))))
    (CallFunction|LevelUp (Utilities|Text|FormatText "Vitality Level: {1}" (.vit_lvl _output_get_2)))
    (CallFunction|SetHPValues false)))

(fn AddSTRxp
  (params (XPyield :type Float%20%28single-precision%29))
  (bind _output_get (Variables|Default|SetAttributeStruct (Utilities|Struct|MakeAttributeStruct (.vit_lvl (Variables|Default|GetAttributeStruct)) (.vit_xp (Variables|Default|GetAttributeStruct)) (.vit_xp_required (Variables|Default|GetAttributeStruct)) (.str_lvl (Variables|Default|GetAttributeStruct)) (+ (.str_xp (Variables|Default|GetAttributeStruct)) XPyield) (.str_xp_required (Variables|Default|GetAttributeStruct)) (.end_lvl (Variables|Default|GetAttributeStruct)) (.end_xp (Variables|Default|GetAttributeStruct)) (.end_xp_required (Variables|Default|GetAttributeStruct)) (.fin_lvl (Variables|Default|GetAttributeStruct)) (.fin_xp (Variables|Default|GetAttributeStruct)) (.fin_xp_required (Variables|Default|GetAttributeStruct)) (.int_lvl (Variables|Default|GetAttributeStruct)) (.int_xp (Variables|Default|GetAttributeStruct)) (.int_xp_required (Variables|Default|GetAttributeStruct)) (.wis_lvl (Variables|Default|GetAttributeStruct)) (.wis_xp (Variables|Default|GetAttributeStruct)) (.wis_xp_required (Variables|Default|GetAttributeStruct)) (.cha_lvl (Variables|Default|GetAttributeStruct)) (.cha_xp (Variables|Default|GetAttributeStruct)) (.cha_xp_required (Variables|Default|GetAttributeStruct)))))
  (if (>= (.str_xp (Variables|Default|GetAttributeStruct)) (.str_xp_required (Variables|Default|GetAttributeStruct)))
    (bind _output_get_2 (Variables|Default|SetAttributeStruct (Utilities|Struct|MakeAttributeStruct (.vit_lvl _output_get) (.vit_xp _output_get) (.vit_xp_required _output_get) (+ (.str_lvl _output_get) 1) 0.0 (Math|Conversions|ToFloat(Integer) (Math|Float|Round (* (.str_xp_required _output_get) (Variables|Default|GetXP_Required_Exponent)))) (.end_lvl _output_get) (.end_xp _output_get) (.end_xp_required _output_get) (.fin_lvl _output_get) (.fin_xp _output_get) (.fin_xp_required _output_get) (.int_lvl _output_get) (.int_xp _output_get) (.int_xp_required _output_get) (.wis_lvl _output_get) (.wis_xp _output_get) (.wis_xp_required _output_get) (.cha_lvl _output_get) (.cha_xp _output_get) (.cha_xp_required _output_get))))
    (CallFunction|LevelUp (Utilities|Text|FormatText "Strength Level: {1}" (.str_lvl _output_get_2)))))

(fn AddENDxp
  (params (XPyield :type Float%20%28single-precision%29))
  (bind _output_get (Variables|Default|SetAttributeStruct (Utilities|Struct|MakeAttributeStruct (.vit_lvl (Variables|Default|GetAttributeStruct)) (.vit_xp (Variables|Default|GetAttributeStruct)) (.vit_xp_required (Variables|Default|GetAttributeStruct)) (.str_lvl (Variables|Default|GetAttributeStruct)) (.str_xp (Variables|Default|GetAttributeStruct)) (.str_xp_required (Variables|Default|GetAttributeStruct)) (.end_lvl (Variables|Default|GetAttributeStruct)) (+ (.end_xp (Variables|Default|GetAttributeStruct)) XPyield) (.end_xp_required (Variables|Default|GetAttributeStruct)) (.fin_lvl (Variables|Default|GetAttributeStruct)) (.fin_xp (Variables|Default|GetAttributeStruct)) (.fin_xp_required (Variables|Default|GetAttributeStruct)) (.int_lvl (Variables|Default|GetAttributeStruct)) (.int_xp (Variables|Default|GetAttributeStruct)) (.int_xp_required (Variables|Default|GetAttributeStruct)) (.wis_lvl (Variables|Default|GetAttributeStruct)) (.wis_xp (Variables|Default|GetAttributeStruct)) (.wis_xp_required (Variables|Default|GetAttributeStruct)) (.cha_lvl (Variables|Default|GetAttributeStruct)) (.cha_xp (Variables|Default|GetAttributeStruct)) (.cha_xp_required (Variables|Default|GetAttributeStruct)))))
  (if (>= (.end_xp (Variables|Default|GetAttributeStruct)) (.end_xp_required (Variables|Default|GetAttributeStruct)))
    (bind _output_get_2 (Variables|Default|SetAttributeStruct (Utilities|Struct|MakeAttributeStruct (.vit_lvl _output_get) (.vit_xp _output_get) (.vit_xp_required _output_get) (.str_lvl _output_get) (.str_xp _output_get) (.str_xp_required _output_get) (+ (.end_lvl _output_get) 1) 0.0 (Math|Conversions|ToFloat(Integer) (Math|Float|Round (* (.end_xp_required _output_get) (Variables|Default|GetXP_Required_Exponent)))) (.fin_lvl _output_get) (.fin_xp _output_get) (.fin_xp_required _output_get) (.int_lvl _output_get) (.int_xp _output_get) (.int_xp_required _output_get) (.wis_lvl _output_get) (.wis_xp _output_get) (.wis_xp_required _output_get) (.cha_lvl _output_get) (.cha_xp _output_get) (.cha_xp_required _output_get))))
    (CallFunction|LevelUp (Utilities|Text|FormatText "Endurance Level: {1}" (.end_lvl _output_get_2)))))

(fn AddFINxp
  (params (XPyield :type Float%20%28single-precision%29))
  (bind _output_get (Variables|Default|SetAttributeStruct (Utilities|Struct|MakeAttributeStruct (.vit_lvl (Variables|Default|GetAttributeStruct)) (.vit_xp (Variables|Default|GetAttributeStruct)) (.vit_xp_required (Variables|Default|GetAttributeStruct)) (.str_lvl (Variables|Default|GetAttributeStruct)) (.str_xp (Variables|Default|GetAttributeStruct)) (.str_xp_required (Variables|Default|GetAttributeStruct)) (.end_lvl (Variables|Default|GetAttributeStruct)) (.end_xp (Variables|Default|GetAttributeStruct)) (.end_xp_required (Variables|Default|GetAttributeStruct)) (.fin_lvl (Variables|Default|GetAttributeStruct)) (+ (.fin_xp (Variables|Default|GetAttributeStruct)) XPyield) (.fin_xp_required (Variables|Default|GetAttributeStruct)) (.int_lvl (Variables|Default|GetAttributeStruct)) (.int_xp (Variables|Default|GetAttributeStruct)) (.int_xp_required (Variables|Default|GetAttributeStruct)) (.wis_lvl (Variables|Default|GetAttributeStruct)) (.wis_xp (Variables|Default|GetAttributeStruct)) (.wis_xp_required (Variables|Default|GetAttributeStruct)) (.cha_lvl (Variables|Default|GetAttributeStruct)) (.cha_xp (Variables|Default|GetAttributeStruct)) (.cha_xp_required (Variables|Default|GetAttributeStruct)))))
  (if (>= (.fin_xp (Variables|Default|GetAttributeStruct)) (.fin_xp_required (Variables|Default|GetAttributeStruct)))
    (bind _output_get_2 (Variables|Default|SetAttributeStruct (Utilities|Struct|MakeAttributeStruct (.vit_lvl _output_get) (.vit_xp _output_get) (.vit_xp_required _output_get) (.str_lvl _output_get) (.str_xp _output_get) (.str_xp_required _output_get) (.end_lvl _output_get) (.end_xp _output_get) (.end_xp_required _output_get) (+ (.fin_lvl _output_get) 1) 0.0 (Math|Conversions|ToFloat(Integer) (Math|Float|Round (* (.fin_xp_required _output_get) (Variables|Default|GetXP_Required_Exponent)))) (.int_lvl _output_get) (.int_xp _output_get) (.int_xp_required _output_get) (.wis_lvl _output_get) (.wis_xp _output_get) (.wis_xp_required _output_get) (.cha_lvl _output_get) (.cha_xp _output_get) (.cha_xp_required _output_get))))
    (CallFunction|LevelUp (Utilities|Text|FormatText "Finesse Level: {1}" (.fin_lvl _output_get_2)))))

(fn AddINTxp
  (params (XPyield :type Float%20%28single-precision%29))
  (bind _output_get (Variables|Default|SetAttributeStruct (Utilities|Struct|MakeAttributeStruct (.vit_lvl (Variables|Default|GetAttributeStruct)) (.vit_xp (Variables|Default|GetAttributeStruct)) (.vit_xp_required (Variables|Default|GetAttributeStruct)) (.str_lvl (Variables|Default|GetAttributeStruct)) (.str_xp (Variables|Default|GetAttributeStruct)) (.str_xp_required (Variables|Default|GetAttributeStruct)) (.end_lvl (Variables|Default|GetAttributeStruct)) (.end_xp (Variables|Default|GetAttributeStruct)) (.end_xp_required (Variables|Default|GetAttributeStruct)) (.fin_lvl (Variables|Default|GetAttributeStruct)) (.fin_xp (Variables|Default|GetAttributeStruct)) (.fin_xp_required (Variables|Default|GetAttributeStruct)) (.int_lvl (Variables|Default|GetAttributeStruct)) (+ (.int_xp (Variables|Default|GetAttributeStruct)) XPyield) (.int_xp_required (Variables|Default|GetAttributeStruct)) (.wis_lvl (Variables|Default|GetAttributeStruct)) (.wis_xp (Variables|Default|GetAttributeStruct)) (.wis_xp_required (Variables|Default|GetAttributeStruct)) (.cha_lvl (Variables|Default|GetAttributeStruct)) (.cha_xp (Variables|Default|GetAttributeStruct)) (.cha_xp_required (Variables|Default|GetAttributeStruct)))))
  (if (>= (.int_xp (Variables|Default|GetAttributeStruct)) (.int_xp_required (Variables|Default|GetAttributeStruct)))
    (bind _output_get_2 (Variables|Default|SetAttributeStruct (Utilities|Struct|MakeAttributeStruct (.vit_lvl _output_get) (.vit_xp _output_get) (.vit_xp_required _output_get) (.str_lvl _output_get) (.str_xp _output_get) (.str_xp_required _output_get) (.end_lvl _output_get) (.end_xp _output_get) (.end_xp_required _output_get) (.fin_lvl _output_get) (.fin_xp _output_get) (.fin_xp_required _output_get) (+ (.int_lvl _output_get) 1) 0.0 (Math|Conversions|ToFloat(Integer) (Math|Float|Round (* (.int_xp_required _output_get) (Variables|Default|GetXP_Required_Exponent)))) (.wis_lvl _output_get) (.wis_xp _output_get) (.wis_xp_required _output_get) (.cha_lvl _output_get) (.cha_xp _output_get) (.cha_xp_required _output_get))))
    (CallFunction|LevelUp (Utilities|Text|FormatText "Intelligence Level: {1}" (.int_lvl _output_get_2)))))

(fn AddWISxp
  (params (XPyield :type Float%20%28single-precision%29))
  (bind _output_get (Variables|Default|SetAttributeStruct (Utilities|Struct|MakeAttributeStruct (.vit_lvl (Variables|Default|GetAttributeStruct)) (.vit_xp (Variables|Default|GetAttributeStruct)) (.vit_xp_required (Variables|Default|GetAttributeStruct)) (.str_lvl (Variables|Default|GetAttributeStruct)) (.str_xp (Variables|Default|GetAttributeStruct)) (.str_xp_required (Variables|Default|GetAttributeStruct)) (.end_lvl (Variables|Default|GetAttributeStruct)) (.end_xp (Variables|Default|GetAttributeStruct)) (.end_xp_required (Variables|Default|GetAttributeStruct)) (.fin_lvl (Variables|Default|GetAttributeStruct)) (.fin_xp (Variables|Default|GetAttributeStruct)) (.fin_xp_required (Variables|Default|GetAttributeStruct)) (.int_lvl (Variables|Default|GetAttributeStruct)) (.int_xp (Variables|Default|GetAttributeStruct)) (.int_xp_required (Variables|Default|GetAttributeStruct)) (.wis_lvl (Variables|Default|GetAttributeStruct)) (+ (.wis_xp (Variables|Default|GetAttributeStruct)) XPyield) (.wis_xp_required (Variables|Default|GetAttributeStruct)) (.cha_lvl (Variables|Default|GetAttributeStruct)) (.cha_xp (Variables|Default|GetAttributeStruct)) (.cha_xp_required (Variables|Default|GetAttributeStruct)))))
  (if (>= (.wis_xp (Variables|Default|GetAttributeStruct)) (.wis_xp_required (Variables|Default|GetAttributeStruct)))
    (bind _output_get_2 (Variables|Default|SetAttributeStruct (Utilities|Struct|MakeAttributeStruct (.vit_lvl _output_get) (.vit_xp _output_get) (.vit_xp_required _output_get) (.str_lvl _output_get) (.str_xp _output_get) (.str_xp_required _output_get) (.end_lvl _output_get) (.end_xp _output_get) (.end_xp_required _output_get) (.fin_lvl _output_get) (.fin_xp _output_get) (.fin_xp_required _output_get) (.int_lvl _output_get) (.int_xp _output_get) (.int_xp_required _output_get) (+ (.wis_lvl _output_get) 1) 0.0 (Math|Conversions|ToFloat(Integer) (Math|Float|Round (* (.wis_xp_required _output_get) (Variables|Default|GetXP_Required_Exponent)))) (.cha_lvl _output_get) (.cha_xp _output_get) (.cha_xp_required _output_get))))
    (CallFunction|LevelUp (Utilities|Text|FormatText "Wisdom Level: {1}" (.wis_lvl _output_get_2)))))

(fn AddCHAxp
  (params (XPyield :type Float%20%28single-precision%29))
  (bind _output_get (Variables|Default|SetAttributeStruct (Utilities|Struct|MakeAttributeStruct (.vit_lvl (Variables|Default|GetAttributeStruct)) (.vit_xp (Variables|Default|GetAttributeStruct)) (.vit_xp_required (Variables|Default|GetAttributeStruct)) (.str_lvl (Variables|Default|GetAttributeStruct)) (.str_xp (Variables|Default|GetAttributeStruct)) (.str_xp_required (Variables|Default|GetAttributeStruct)) (.end_lvl (Variables|Default|GetAttributeStruct)) (.end_xp (Variables|Default|GetAttributeStruct)) (.end_xp_required (Variables|Default|GetAttributeStruct)) (.fin_lvl (Variables|Default|GetAttributeStruct)) (.fin_xp (Variables|Default|GetAttributeStruct)) (.fin_xp_required (Variables|Default|GetAttributeStruct)) (.int_lvl (Variables|Default|GetAttributeStruct)) (.int_xp (Variables|Default|GetAttributeStruct)) (.int_xp_required (Variables|Default|GetAttributeStruct)) (.wis_lvl (Variables|Default|GetAttributeStruct)) (.wis_xp (Variables|Default|GetAttributeStruct)) (.wis_xp_required (Variables|Default|GetAttributeStruct)) (.cha_lvl (Variables|Default|GetAttributeStruct)) (+ (.cha_xp (Variables|Default|GetAttributeStruct)) XPyield) (.cha_xp_required (Variables|Default|GetAttributeStruct)))))
  (if (>= (.cha_xp (Variables|Default|GetAttributeStruct)) (.cha_xp_required (Variables|Default|GetAttributeStruct)))
    (bind _output_get_2 (Variables|Default|SetAttributeStruct (Utilities|Struct|MakeAttributeStruct (.vit_lvl _output_get) (.vit_xp _output_get) (.vit_xp_required _output_get) (.str_lvl _output_get) (.str_xp _output_get) (.str_xp_required _output_get) (.end_lvl _output_get) (.end_xp _output_get) (.end_xp_required _output_get) (.fin_lvl _output_get) (.fin_xp _output_get) (.fin_xp_required _output_get) (.int_lvl _output_get) (.int_xp _output_get) (.int_xp_required _output_get) (.wis_lvl _output_get) (.wis_xp _output_get) (.wis_xp_required _output_get) (+ (.cha_lvl _output_get) 1) 0.0 (Math|Conversions|ToFloat(Integer) (Math|Float|Round (* (.cha_xp_required _output_get) (Variables|Default|GetXP_Required_Exponent)))))))
    (CallFunction|LevelUp (Utilities|Text|FormatText "Charisma Level: {1}" (.cha_lvl _output_get_2)))))

(fn SetHPValues
  (params (HealToMaxHP? :type Boolean))
  (bind _attributestruct (Variables|Default|GetAttributeStruct))
  (bind _as_timeless_character (Variables|Default|GetAs%20Timeless%20Character))
  (bind _returnvalue (* (.vit_lvl _attributestruct) 5))
  (bind _returnvalue_2 (Math|Conversions|ToFloat(Integer) _returnvalue))
  (bind _output_get (Variables|/Game/Blueprints/TimelessCharacter.TimelessCharacter_C|SetMaxHealth _as_timeless_character (+ _returnvalue_2 1e+02)))
  (LocalVariables|SetHPscaleMOD _returnvalue_2)
  (if HealToMaxHP?
    (Variables|/Game/Blueprints/TimelessCharacter.TimelessCharacter_C|SetHealth _as_timeless_character _output_get))
  (Default|CallScaleHPbar (LocalVariables|GetHPscaleMOD)))