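; Arrow projectile that sticks into what it hits and damages NPCs on behalf of the player.
; A particle trail runs between tip and end sockets from BeginPlay until the first valid sphere overlap, which ignores itself, the player, the instigator and other arrows.
; On impact it stops movement, attaches to the hit actor and disables collision.
; One-time damage requires an NPC_Parent with the TakesDamage gameplay tag, and awards the player combat skill experience.
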(event OnComponentBeginOverlap(Sphere)
  (params (OverlappedComponent :type Primitive%20Component%20Object%20Reference) (OtherActor :type Actor%20Object%20Reference) (OtherComp :type Primitive%20Component%20Object%20Reference) (OtherBodyIndex :type Integer) (bFromSweep :type Boolean) (SweepResult :type Hit%20Result%20Structure%20%28by%20ref%29))
  (bind _hitactor (Collision|BreakHitResult SweepResult))
  (if (Math|Boolean|ANDBoolean (!= self OtherActor) (!= (Variables|Default|GetPlayerCharacter) OtherActor) (!= (Game|GetInstigator) OtherActor) (!= (Utilities|GetClass OtherActor) "ArrowProjectile_C"))
    (Components|Activation|Deactivate (Variables|Default|GetProjectileMovement))
    (CallFunction|EndTrail)
    (Transformation|AttachActorToActor self _hitactor "None" "KeepWorld" "KeepWorld" "KeepWorld" true)
    (Collision|SetCollisionEnabled (Variables|Default|GetSphere) "NoCollision")
    (Utilities|FlowControl|DoN 1
      (:Exit
        (bind _asnpc_parent (Utilities|Casting|CastToNPC_Parent _hitactor))
        (if (GameplayTags|DoesContainerMatchTagQuery (Variables|/Game/Blueprints/NPCs/NPC_Parent.NPC_Parent_C|GetGameplayTags _asnpc_parent) (GameplayTags|MakeGameplayTagQuery "(TokenStreamVersion=0,TagDictionary=((TagName=\"TakesDamage\")),QueryTokenStream=(0,1,1,1,0),UserDescription=\"\",AutoDescription=\" ANY( TakesDamage )\")"))
          (bind _returnvalue (Game|Damage|ApplyDamage _hitactor (Variables|Default|GetDamage) 0 (Variables|Default|GetPlayerCharacter) "/Script/Engine.DamageType"))
          (Default|CombatSkillExp (Variables|Default|GetPlayerCharacter) _returnvalue (Variables|Default|GetAttributeUsed)))))))

(event Custom|EndTrail
  (Effects|Particles|Trails|EndTrails (Variables|Default|GetP_Trail)))

(event EventBeginPlay
  (Effects|Particles|Trails|BeginTrails (Variables|Default|GetP_Trail) "ArrowTip" "ArrowEnd" "ETrailWidthMode_FromFirst" 0.6))

(fn ConstructionScript)