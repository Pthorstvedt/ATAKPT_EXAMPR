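; Stand-in actor that mirrors the player character's skeletal mesh, apparently for a 3D capture in the inventory's character equipment view.
; On BeginPlay it casts player 0 to TimelessCharacter and stores it as both SourceActor and a typed reference.
; UpdateMesh then copies that character's current skeletal mesh asset onto its own SkeletalMesh component, reinitializing the pose.
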(event Custom|UpdateMesh
  (Class|SkinnedMeshComponent|SetSkeletalMesh (Variables|Default|GetSkeletalMesh) (Variables|/Script/Engine.SkinnedMeshComponent|GetSkeletalMesh (Variables|/Script/Engine.Character|GetMesh (Variables|Default|GetAs%20Timeless%20Character))) true))

(event EventBeginPlay
  (bind _astimeless_character (Utilities|Casting|CastToTimelessCharacter (Game|GetPlayerCharacter 0)))
  (Variables|Default|SetSourceActor _astimeless_character)
  (Variables|Default|SetAs%20Timeless%20Character _astimeless_character)
  (CallFunction|UpdateMesh))

(fn ConstructionScript)