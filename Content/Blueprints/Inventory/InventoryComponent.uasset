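; Inventory and equipment component that manages stackable items in fixed slots, toggles the inventory widget and restores saved equipment on BeginPlay.
; Adding fills partial stacks before empty slots and notifies quest objectives for non-NPC pickups; removal can span stacks.
; Equipping returns the old item to inventory, then recalculates TimelessCharacter armor and damage from all slots.
; Equipment meshes are copied from temporary actors spawned far below the origin.
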(event Custom|UpdateStats
  (bind _as_timeless_character (Variables|Default|GetAs%20Timeless%20Character))
  ;[1 1 1] Reset Stats before calculation to not increment
  (Variables|/Game/Blueprints/TimelessCharacter.TimelessCharacter_C|SetTotalArmor _as_timeless_character 0.0)
  (Variables|/Game/Blueprints/TimelessCharacter.TimelessCharacter_C|SetTotalArmorWeight _as_timeless_character 0.0)
  (Variables|/Game/Blueprints/TimelessCharacter.TimelessCharacter_C|SetMainHandDamage _as_timeless_character 0.0)
  (Variables|/Game/Blueprints/TimelessCharacter.TimelessCharacter_C|SetOffHandDamage _as_timeless_character 0.0)
  (Variables|/Game/Blueprints/TimelessCharacter.TimelessCharacter_C|SetRangedDamage _as_timeless_character 0.0)
  (Variables|/Game/Blueprints/TimelessCharacter.TimelessCharacter_C|SetAmmunitionDamage _as_timeless_character 0.0)
  (bind _keys (Utilities|Map|Keys (Variables|Default|GetEquippedSlots)))
  (for _array_element _keys
    (CallFunction|UpdateStatsforEach _array_element)))

(event EventBeginPlay
  (CallFunction|PrepareInventory)
  (bind _astimeless_character (Utilities|Casting|CastToTimelessCharacter (Components|GetOwner)))
  (Variables|Default|SetAs%20Timeless%20Character _astimeless_character)
  (bind _astimeless_instance (Utilities|Casting|CastToTimelessInstance (Game|GetGameInstance)))
  ;[1 1 1] Equips items from save
  (bind _keys (Utilities|Map|Keys (Variables|/Game/Blueprints/SaveGameObject.SaveGameObject_C|GetPlayerEquipped_Save (Variables|/Game/Blueprints/TimelessInstance.TimelessInstance_C|GetSaveGameData _astimeless_instance))))
  (for _array_element _keys
    (if (.ReturnValue (Utilities|Map|Find (Variables|/Game/Blueprints/SaveGameObject.SaveGameObject_C|GetPlayerEquipped_Save (Variables|/Game/Blueprints/TimelessInstance.TimelessInstance_C|GetSaveGameData _astimeless_instance)) _array_element))
      (CallFunction|EquiptoSlot _array_element (.ItemStructure (Utilities|GetClassDefaults (.Class (Utilities|Struct|BreakItemStruct (.Value (Utilities|Map|Find (Variables|/Game/Blueprints/SaveGameObject.SaveGameObject_C|GetPlayerEquipped_Save (Variables|/Game/Blueprints/TimelessInstance.TimelessInstance_C|GetSaveGameData _astimeless_instance)) _array_element))))))))))

(fn ToggleInventory
  (bind _returnvalue (Game|GetPlayerController 0))
  (bind _returnvalue_2 (Game|GetPlayerController 0))
  (Variables|Default|GetInventoryWindow
    (:then
      (Widget|RemovefromParent (Variables|Default|GetInventoryWindow))
      (Variables|Default|SetInventoryWindow 0)
      (Input|SetInputModeGameOnly _returnvalue_2)
      (Variables|/Script/Engine.PlayerController|SetbShowMouseCursor _returnvalue_2 false))
    (:else
      (CallFunction|PrepareInventory)
      (bind _returnvalue_3 (UserInterface|CreateWidget "/Game/Blueprints/UI/InventoryWindow.InventoryWindow_C" 0 self (Variables|Default|GetInventoryName)))
      (Variables|Default|SetInventoryWindow _returnvalue_3)
      (bind _astimeless_player_controller (Utilities|Casting|CastToTimeless_PlayerController (Game|GetPlayerController 0)))
      (bind _returnvalue_4 (Class|CanvasPanel|AddChildtoCanvas (Variables|/Game/Blueprints/UI/HUD.HUD_C|GetHudCanvas (Variables|/Game/Blueprints/Timeless_PlayerController.Timeless_PlayerController_C|GetHUDwidget _astimeless_player_controller)) (Variables|Default|GetInventoryWindow)))
      (Class|CanvasPanelSlot|SetAutoSize _returnvalue_4 true)
      (Class|CanvasPanelSlot|SetAlignment _returnvalue_4 "(X=0.500000,Y=0.500000)")
      (Class|CanvasPanelSlot|SetAnchors _returnvalue_4 (Utilities|Struct|MakeAnchors "(X=0.500000,Y=0.500000)" "(X=0.500000,Y=0.500000)"))
      (Class|CanvasPanelSlot|SetPosition _returnvalue_4 (Variables|Default|GetPosition))
      (Input|SetInputModeGameandUI _returnvalue (Variables|Default|GetInventoryWindow) "LockInFullscreen" false)
      (Variables|/Script/Engine.PlayerController|SetbShowMouseCursor _returnvalue true))))

(fn AddtoInventory
  (params (ContentToAdd :type Slot%20Struct%20Structure) (IsNPC? :type Boolean))
  (if (.isstackable? (.itemstructure ContentToAdd))
    (bind _stackindex (Utilities|HasPartialStack ContentToAdd)
      (:True
        (bind _success (CallFunction|AddtoStack ContentToAdd _stackindex))
        (LocalVariables|SetGreatSuccess _success))
      (:False
        (bind _success_2 (CallFunction|CreateStack ContentToAdd :!label _label))
        (LocalVariables|SetGreatSuccess _success_2)))
    (else
      (goto _label)))
  (if (LocalVariables|GetGreatSuccess)
    (if (not IsNPC?)
      ;[1 1 1] Checks if looted item is part of a quest
      (Default|CheckCollectionObjective (Variables|/Game/Blueprints/TimelessCharacter.TimelessCharacter_C|GetQuestLogComponent (Variables|Default|GetAs%20Timeless%20Character)) (.itemstructure ContentToAdd))
      (Audio|PlaySound2D "/Game/Bubbyfolder/BestFolder/Sound_Effects/Item_Equiptment/FG_Item_Pickup_Leather_Armor.FG_Item_Pickup_Leather_Armor" 1.0 1.0 0.0 0 0)
      (return (LocalVariables|GetGreatSuccess)))
    (else
      (return (LocalVariables|GetGreatSuccess)))))

(fn PrepareInventory
  (Utilities|Array|Resize (Variables|Default|GetInventory) (Variables|Default|GetNumberOfSlots))
  (for (_array_element _array_index) (Variables|Default|GetInventory)
    (if (not (== (.Class (Utilities|Struct|BreakItemStruct (.itemstructure _array_element))) 0))
      (Utilities|Array|SetArrayElem (Variables|Default|GetInventory) _array_index (Utilities|Struct|MakeSlotStruct (.ItemStructure (Utilities|GetClassDefaults (.Class (Utilities|Struct|BreakItemStruct (.itemstructure _array_element))))) (.quantity _array_element))))))

(fn CreateStack
  (params (ContentToAdd :type Slot%20Struct%20Structure))
  (bind (_array_element _array_index) (Utilities|Array|ForEachLoopwithBreak (Variables|Default|GetInventory) :!label _label)
    (:LoopBody
      (if (<= (.quantity _array_element) 0)
        (LocalVariables|SetHasSpace true)
        (LocalVariables|SetIdentifiedIndex _array_index)
        (goto _label Break)))
    (:Completed
      (if (LocalVariables|GetHasSpace)
        (Utilities|Array|SetArrayElem (Variables|Default|GetInventory) (LocalVariables|GetIdentifiedIndex) ContentToAdd)
        (return (LocalVariables|GetHasSpace))
        (else
          (return false))))))

(fn AddtoStack
  (params (SlotStructure :type Slot%20Struct%20Structure) (SlotIndex :type Integer))
  (bind _inventory (Variables|Default|GetInventory))
  (bind _inventory_2 (Variables|Default|GetInventory))
  (bind _maxstacksize (Utilities|Struct|BreakItemStruct (.itemstructure SlotStructure)))
  (bind _output (Utilities|Array|Get(acopy) _inventory SlotIndex))
  (bind _output_2 (Utilities|Array|Get(acopy) _inventory_2 SlotIndex))
  (bind _output_get (LocalVariables|SetCurrentQuantity (.quantity _output)))
  (if (> (+ _output_get (.Quantity (Utilities|Struct|BreakSlotStruct SlotStructure))) (.maxstacksize (.itemstructure _output)))
    (Utilities|Array|SetArrayElem (Variables|Default|GetInventory) SlotIndex (Utilities|Struct|MakeSlotStruct (.itemstructure SlotStructure) _maxstacksize))
    (CallFunction|AddtoInventory (Utilities|Struct|MakeSlotStruct (.itemstructure SlotStructure) (- (.quantity SlotStructure) (- _maxstacksize (LocalVariables|GetCurrentQuantity)))) false)
    (else
      (Utilities|Array|SetArrayElem _inventory_2 SlotIndex (Utilities|Struct|MakeSlotStruct (.itemstructure _output_2) (+ (.quantity _output_2) (.quantity SlotStructure))))))
  (return true))

(fn InventoryQuery
  (params (QueryItem :type 0%20Item%20Parent%20Class%20Reference) (QueryAmount :type Integer))
  (bind _array_element (Utilities|Array|ForEachLoopwithBreak (Variables|Default|GetInventory))
    (:LoopBody
      (if (== (.Class (Utilities|Struct|BreakItemStruct (.itemstructure _array_element))) QueryItem)
        (LocalVariables|SetRunningTotal (+ (.quantity _array_element) (LocalVariables|GetRunningTotal)))))
    (:Completed
      (return (>= (LocalVariables|GetRunningTotal) QueryAmount) (LocalVariables|GetRunningTotal)))))

(fn EquiptoSlot
  (params (ItemSlot :type E_SlotType%20Enum :default "NewEnumerator0") (ItemStruct :type Item%20Struct%20Structure))
  (bind _equippedslots (Variables|Default|GetEquippedSlots))
  ;[1 1 1] Checks if slot is empty
  (if (!= (.class (.Value (Utilities|Map|Find _equippedslots ItemSlot))) 0)
    (bind _success (CallFunction|AddtoInventory (Utilities|Struct|MakeSlotStruct (.Value (Utilities|Map|Find _equippedslots ItemSlot)) 1) false))
    (if _success
      (Utilities|Map|Add _equippedslots ItemSlot ItemStruct :!label _label)
      (CallFunction|UpdateStats)
      (CallFunction|UpdateStaticMesh ItemSlot ItemStruct)
      (CallFunction|RemovefromInventory ItemStruct 1))
    (else
      (goto _label))))

(fn UpdateStatsforEach
  (params (SlotType :type E_SlotType%20Enum :default "NewEnumerator0"))
  (bind _equippedslots (Variables|Default|GetEquippedSlots))
  (bind _as_timeless_character (Variables|Default|GetAs%20Timeless%20Character))
  (bind (_value _returnvalue) (Utilities|Map|Find _equippedslots SlotType))
  (if _returnvalue
    (switch Utilities|FlowControl|Switch|SwitchonE_SlotType (.slottype _value)
      (:NewEnumerator2
        (Variables|/Game/Blueprints/TimelessCharacter.TimelessCharacter_C|SetTotalArmor _as_timeless_character (+ (Variables|/Game/Blueprints/TimelessCharacter.TimelessCharacter_C|GetTotalArmor _as_timeless_character) (.basearmor (.armorstruct _value))) :!label _label)
        (Variables|/Game/Blueprints/TimelessCharacter.TimelessCharacter_C|SetTotalArmorWeight _as_timeless_character (+ (Variables|/Game/Blueprints/TimelessCharacter.TimelessCharacter_C|GetTotalArmorWeight _as_timeless_character) (.weight (.armorstruct _value)))))
      (:NewEnumerator3
        (goto _label))
      (:NewEnumerator4
        (goto _label))
      (:NewEnumerator5
        (goto _label))
      (:NewEnumerator6
        (goto _label))
      (:NewEnumerator7
        (goto _label))
      (:NewEnumerator8
        (goto _label))
      (:NewEnumerator9
        (Variables|/Game/Blueprints/TimelessCharacter.TimelessCharacter_C|SetMainHandDamage _as_timeless_character (.basedamage (.weaponstruct _value)))
        (Variables|/Game/Blueprints/TimelessCharacter.TimelessCharacter_C|SetMainHandWeight _as_timeless_character (.weight (.weaponstruct _value))))
      (:NewEnumerator10
        (Variables|/Game/Blueprints/TimelessCharacter.TimelessCharacter_C|SetOffHandDamage _as_timeless_character (.basedamage (.weaponstruct _value))))
      (:NewEnumerator11
        (Variables|/Game/Blueprints/TimelessCharacter.TimelessCharacter_C|SetRangedDamage _as_timeless_character (.basedamage (.weaponstruct _value))))
      (:NewEnumerator13
        (Variables|/Game/Blueprints/TimelessCharacter.TimelessCharacter_C|SetAmmunitionDamage _as_timeless_character (.basedamage (.weaponstruct _value)))))))

(fn UpdateStaticMesh
  (params (E_SlotType :type E_SlotType%20Enum :default "NewEnumerator0") (ItemStruct :type Item%20Struct%20Structure))
  (bind _as_timeless_character (Variables|Default|GetAs%20Timeless%20Character))
  (if (not (== (.class ItemStruct) 0))
    (bind _returnvalue (Game|SpawnActorfromClass (.class ItemStruct) (Math|Transform|MakeTransform "0, 0,-10000.000000") "AlwaysSpawn" 0 0))
    (switch Utilities|FlowControl|Switch|SwitchonE_SlotType E_SlotType
      (:NewEnumerator2
        (Components|StaticMesh|SetStaticMesh (Variables|/Game/Blueprints/TimelessCharacter.TimelessCharacter_C|GetSM_Helmet (Variables|Default|GetAs%20Timeless%20Character)) (Variables|/Script/Engine.StaticMeshComponent|GetStaticMesh (Variables|/Game/Blueprints/Inventory/Items/0_Item_Parent.0_Item_Parent_C|GetStaticMesh _returnvalue)))
        (Actor|DestroyActor _returnvalue :!label _label))
      (:NewEnumerator3
        (Components|StaticMesh|SetStaticMesh (Variables|/Game/Blueprints/TimelessCharacter.TimelessCharacter_C|GetSM_L_Shoulder _as_timeless_character) (Variables|/Script/Engine.StaticMeshComponent|GetStaticMesh (Variables|/Game/Blueprints/Inventory/Items/0_Item_Parent.0_Item_Parent_C|GetStaticMesh _returnvalue)))
        (Components|StaticMesh|SetStaticMesh (Variables|/Game/Blueprints/TimelessCharacter.TimelessCharacter_C|GetSM_R_Shoulder _as_timeless_character) (Variables|/Script/Engine.StaticMeshComponent|GetStaticMesh (Variables|/Game/Blueprints/Inventory/Items/0_Item_Parent.0_Item_Parent_C|GetStaticMesh _returnvalue)))
        (goto _label))
      (:NewEnumerator9
        (Components|StaticMesh|SetStaticMesh (Variables|/Game/Blueprints/TimelessCharacter.TimelessCharacter_C|GetSM_MainHand (Variables|Default|GetAs%20Timeless%20Character)) (Variables|/Script/Engine.StaticMeshComponent|GetStaticMesh (Variables|/Game/Blueprints/Inventory/Items/0_Item_Parent.0_Item_Parent_C|GetStaticMesh _returnvalue))))
      (:NewEnumerator11
        (Components|StaticMesh|SetStaticMesh (Variables|/Game/Blueprints/TimelessCharacter.TimelessCharacter_C|GetSM_Ranged (Variables|Default|GetAs%20Timeless%20Character)) (Variables|/Script/Engine.StaticMeshComponent|GetStaticMesh (Variables|/Game/Blueprints/Inventory/Items/0_Item_Parent.0_Item_Parent_C|GetStaticMesh _returnvalue))))
      (:NewEnumerator13
        (Components|StaticMesh|SetStaticMesh (Variables|/Game/Blueprints/TimelessCharacter.TimelessCharacter_C|GetSM_Ammunition (Variables|Default|GetAs%20Timeless%20Character)) (Variables|/Script/Engine.StaticMeshComponent|GetStaticMesh (Variables|/Game/Blueprints/Inventory/Items/0_Item_Parent.0_Item_Parent_C|GetStaticMesh _returnvalue)))))))

(fn RemovefromInventory
  (params (ItemToRemove :type Item%20Struct%20Structure) (AmountToRemove :type Integer))
  (bind _inventory (Variables|Default|GetInventory))
  (bind _hasitems_ (CallFunction|InventoryQuery (.class ItemToRemove) AmountToRemove))
  (if _hasitems_
    (bind (_stackindex _stackamount) (Utilities|HasEnoughinStack (Utilities|Struct|MakeSlotStruct ItemToRemove (- AmountToRemove (LocalVariables|GetAmountRemoved))) :!label _label)
      (:True
        (if (< (- _stackamount (- AmountToRemove (LocalVariables|GetAmountRemoved))) 1)
          (Utilities|Array|SetArrayElem _inventory _stackindex (Utilities|Struct|MakeSlotStruct "(Name_29_00796564423EB52D726E3DBCF4F29323=NSLOCTEXT(\"[36DF52C843BB6C9B127C9DA59A802730]\", \"E040654F491082625553D79686D30EE4\", \"[Name]\"),isStackable?_12_F7A4EAA748B70F9A6C6273968A0B582D=False,Thumbnail_28_BA30AB214C22F7CD5433DF94647B8A75=None,Description_27_E99B604A40B7456F4C575B92B78D8813=NSLOCTEXT(\"[36DF52C843BB6C9B127C9DA59A802730]\", \"8D36C17A4901B3C719239B9751249961\", \"[Description]\"),isConsumable?_15_ADB62D334BB6D704D5B82FAF5237257D=False,MaxStackSize_26_0D71056D47F541A2BBF7A893838E1244=4,Class_25_C64339F845C2BD154376DCB455267CD9=None,isEquippable?_19_CD66620840F738508F9E38ABFADB0955=False,ItemType_24_0D9AF6814E8F3F03131ADBB4FEF8B018=\"[Type]\",isCraftingMat?_21_544EECCA45018C3BF0DE56A68489BF08=False,Value_23_2E649CE144063770BEFF698870D4F4AB=1,SlotType_33_704921BF428C2C1EAAE7AB96D5EBB702=NewEnumerator0,WeaponStruct_38_9491AAF44606F1AF50DF788E9AF8511B=(BaseDamage_2_F93726D146850571D958BBAE63EA6C53=0.000000,Weight_4_08CDD7ED4A0AA1954142808BA4672851=0.000000,WeaponType_7_BF21E729482D8431945E8DBD9682C42A=NewEnumerator13,Rarity_18_32D89F224AA73CF41ECD32885B907E4A=NewEnumerator0,AttributeUsed_21_CE9E82E746BC149BD2EDACADC3B19A6A=NewEnumerator0,DamageType_10_8441BCAA48CE69B6E55500B6B92AC587=None),ArmorStruct_39_0B58301F46CDC7CBA6819FA98E26351D=(BaseArmor_2_3D8CD27640313C513BA09D8A34A69A39=0.000000,Weight_4_F33405D34A91E1713A93CE98FE0760F7=0.000000,Rarity_7_E15031AB44AD66CBAFE789BB4E0B6543=NewEnumerator0))" 0))
          (else
            (Utilities|Array|SetArrayElem _inventory _stackindex (Utilities|Struct|MakeSlotStruct ItemToRemove (- _stackamount (- AmountToRemove (LocalVariables|GetAmountRemoved)))))))
        (Variables|Default|GetInventoryWindow
          (:then
            (CallFunction|ToggleInventory)
            (CallFunction|ToggleInventory))
          (:else)))
      (:False
        (Utilities|Array|SetArrayElem _inventory _stackindex (Utilities|Struct|MakeSlotStruct "(Name_29_00796564423EB52D726E3DBCF4F29323=NSLOCTEXT(\"[36DF52C843BB6C9B127C9DA59A802730]\", \"7C78379E476E00CF0A4F0DBC00C712E9\", \"[Name]\"),isStackable?_12_F7A4EAA748B70F9A6C6273968A0B582D=False,Thumbnail_28_BA30AB214C22F7CD5433DF94647B8A75=None,Description_27_E99B604A40B7456F4C575B92B78D8813=NSLOCTEXT(\"[36DF52C843BB6C9B127C9DA59A802730]\", \"865028AF4BC17258D15A4D8A3EC5933C\", \"[Description]\"),isConsumable?_15_ADB62D334BB6D704D5B82FAF5237257D=False,MaxStackSize_26_0D71056D47F541A2BBF7A893838E1244=4,Class_25_C64339F845C2BD154376DCB455267CD9=None,isEquippable?_19_CD66620840F738508F9E38ABFADB0955=False,ItemType_24_0D9AF6814E8F3F03131ADBB4FEF8B018=\"[Type]\",isCraftingMat?_21_544EECCA45018C3BF0DE56A68489BF08=False,Value_23_2E649CE144063770BEFF698870D4F4AB=1,SlotType_33_704921BF428C2C1EAAE7AB96D5EBB702=NewEnumerator0,WeaponStruct_38_9491AAF44606F1AF50DF788E9AF8511B=(BaseDamage_2_F93726D146850571D958BBAE63EA6C53=0.000000,Weight_4_08CDD7ED4A0AA1954142808BA4672851=0.000000,WeaponType_7_BF21E729482D8431945E8DBD9682C42A=NewEnumerator13,Rarity_18_32D89F224AA73CF41ECD32885B907E4A=NewEnumerator0,AttributeUsed_21_CE9E82E746BC149BD2EDACADC3B19A6A=NewEnumerator0,DamageType_10_8441BCAA48CE69B6E55500B6B92AC587=None),ArmorStruct_39_0B58301F46CDC7CBA6819FA98E26351D=(BaseArmor_2_3D8CD27640313C513BA09D8A34A69A39=0.000000,Weight_4_F33405D34A91E1713A93CE98FE0760F7=0.000000,Rarity_7_E15031AB44AD66CBAFE789BB4E0B6543=NewEnumerator0))" 0))
        (bind _output_get (LocalVariables|SetAmountRemoved (+ _stackamount (LocalVariables|GetAmountRemoved))))
        (if (< _output_get AmountToRemove)
          (goto _label))))))