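; Gavin NPC Blueprint that reacts when a character interacts with him by approaching them and starting his quest behavior.
; On Interact it gets its AI_Parent controller, focuses on the interactor and moves to them.
; When the move's then output fires, the controller's QuestNumber selects whether to run the GavinsQuest or GavinsSecondQuest behavior tree.
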(event EventBeginPlay
  (|CallParentFunction) ; This node is disabled and will not be called.\nDrag off pins to build functionality.
)

(event EventInteract
  (params (Interactor :type Actor%20Object%20Reference))
  (bind _asai_parent (Utilities|Casting|CastToAI_Parent (AI|GetAIController self)))
  (bind _output_get (Variables|Default|SetAs%20AI%20Parent_0 _asai_parent))
  (AI|SetFocus _output_get Interactor)
  (AI|AIMoveTo _output_get "0, 0, 0" Interactor 2.5 "Default" "Default" true false
    (:then
      (switch int (Variables|/Game/Blueprints/NPCs/AI_Parent.AI_Parent_C|GetQuestNumber _output_get)
        (:0
          (AI|RunBehaviorTree (Variables|Default|GetAs%20AI%20Parent_0) (Variables|Default|GetGavinsQuest)))
        (:1
          (AI|RunBehaviorTree (Variables|Default|GetAs%20AI%20Parent_0) (Variables|Default|GetGavinsSecondQuest)))))))

(fn ConstructionScript
  (|CallParentFunction))