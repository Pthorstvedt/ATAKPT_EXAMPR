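; Behavior tree task that advances an NPC's patrol point index in the Blackboard.
; It casts the controlled pawn to NPC_Parent and compares the BBPathIndex key with the length of its PatrolPath's PathPoints.
; The index increments by one and wraps to zero after the last point, then the task finishes successfully.
; A failed cast or an index beyond the last point never calls FinishExecute.
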(event EventReceiveExecuteAI
  (params (OwnerController :type AI%20Controller%20Object%20Reference) (ControlledPawn :type Pawn%20Object%20Reference))
  (bind _bb_pathindex (Variables|Default|GetBB_PathIndex))
  (bind _returnvalue (Class|BTFunctionLibrary|GetBlackboardValueasInt _bb_pathindex))
  (bind _returnvalue_2 (+ _returnvalue 1))
  (bind _asnpc_parent (Utilities|Casting|CastToNPC_Parent ControlledPawn))
  ;[1 1 1] If Path index is equal to amount  of points => set Path index to 0
  ; Else=> Increment Path Index
  (if (== _returnvalue (- (Utilities|Array|Length (Variables|/Game/Blueprints/NPCs/PatrolPath.PatrolPath_C|GetPathPoints (Variables|/Game/Blueprints/NPCs/NPC_Parent.NPC_Parent_C|GetPatrolPath _asnpc_parent))) 1))
    (Class|BTFunctionLibrary|SetBlackboardValueasInt (Variables|Default|GetBB_PathIndex))
    (AI|BehaviorTree|FinishExecute true :!label _label)
    (elif (<= _returnvalue_2 (- (Utilities|Array|Length (Variables|/Game/Blueprints/NPCs/PatrolPath.PatrolPath_C|GetPathPoints (Variables|/Game/Blueprints/NPCs/NPC_Parent.NPC_Parent_C|GetPatrolPath _asnpc_parent))) 1))
      (Class|BTFunctionLibrary|SetBlackboardValueasInt (Variables|Default|GetBB_PathIndex) _returnvalue_2)
      (goto _label))))