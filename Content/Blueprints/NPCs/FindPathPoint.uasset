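; FindPathPoint is a behavior tree task that gives a patrolling NPC the location of its current patrol point.
; It reads the index from the blackboard, looks up that point on the NPC_Parent's PatrolPath and transforms it from path-local to world space.
; It writes the result to the path vector key and finishes successfully.
; A failed cast or invalid path never calls FinishExecute, leaving the task running.
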(event EventReceiveExecuteAI
  (params (OwnerController :type AI%20Controller%20Object%20Reference) (ControlledPawn :type Pawn%20Object%20Reference))
  ;[1 1 1] Find path point from index
  (bind _asnpc_parent (Utilities|Casting|CastToNPC_Parent ControlledPawn))
  (bind _patrolpath (Variables|/Game/Blueprints/NPCs/NPC_Parent.NPC_Parent_C|GetPatrolPath _asnpc_parent)
    (:then
      (AI|BehaviorTree|SetBlackboardValueasVector (Variables|Default|GetBB_PathVector) (Math|Transform|TransformLocation (Transformation|GetActorTransform _patrolpath) (Utilities|Array|Get(acopy) (Variables|/Game/Blueprints/NPCs/PatrolPath.PatrolPath_C|GetPathPoints _patrolpath) (Class|BTFunctionLibrary|GetBlackboardValueasInt (Variables|Default|GetBB_PathIndex)))))
      (AI|BehaviorTree|FinishExecute true))
    (:else)))