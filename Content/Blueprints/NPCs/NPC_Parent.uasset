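; Base NPC Blueprint providing health, death, loot and player interaction, with empty hooks for animations, looting and animal sounds and attacks.
; Damage lowers health and spawns floating text; death notifies the hostile or animal AI controller, updates the player's kill objective and rolls the loot table into the inventory.
; Interacting moves a living NPC to the interactor, then runs a quest-selected behavior tree, or opens a corpse's inventory.
; Sphere overlap toggles outline highlighting.
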(event OnComponentEndOverlap(InteractSphere)
  (params (OverlappedComponent :type Primitive%20Component%20Object%20Reference) (OtherActor :type Actor%20Object%20Reference) (OtherComp :type Primitive%20Component%20Object%20Reference) (OtherBodyIndex :type Integer))
  (bind _mesh (Variables|Character|GetMesh))
  (bind _inventorycomponent (Variables|Default|GetInventoryComponent))
  (Rendering|SetRenderCustomDepth _mesh false)
  (Rendering|SetCustomDepthStencilValue _mesh 0)
  (Variables|/Game/Blueprints/Inventory/InventoryComponent.InventoryComponent_C|GetInventoryWindow _inventorycomponent
    (:then
      (Default|ToggleInventory _inventorycomponent))
    (:else)))

(event OnComponentBeginOverlap(InteractSphere)
  (params (OverlappedComponent :type Primitive%20Component%20Object%20Reference) (OtherActor :type Actor%20Object%20Reference) (OtherComp :type Primitive%20Component%20Object%20Reference) (OtherBodyIndex :type Integer) (bFromSweep :type Boolean) (SweepResult :type Hit%20Result%20Structure%20%28by%20ref%29))
  (bind _mesh (Variables|Character|GetMesh))
  (Rendering|SetRenderCustomDepth _mesh true)
  (Rendering|SetCustomDepthStencilValue _mesh 2))

(event Custom|GenerateLoot
  (Variables|/Game/Blueprints/Inventory/InventoryComponent.InventoryComponent_C|SetInventoryName (Variables|Default|GetInventoryComponent) (Variables|Default|GetNameType))
  (CallFunction|RollLootTable)
  (Collision|SetCollisionEnabled (Variables|Default|GetInteractSphere) "QueryOnly")
  (CallFunction|PlayDeathAnimation))

(event Custom|DeadSpawn
  (bind _self self)
  (bind _returnvalue (AI|GetAIController _self))
  (bind _asai_hostile (Utilities|Casting|CastToAI_Hostile _returnvalue)
    (:then
      (Default|EventDie _asai_hostile))
    (:CastFailed
      (bind _asai_animals (Utilities|Casting|CastToAI_Animals _returnvalue))
      (Default|EventDie _asai_animals)))
  (Collision|SetCollisionEnabled (Variables|Collision|GetCapsuleComponent) "NoCollision")
  (Default|CheckKillObjective (Variables|/Game/Blueprints/TimelessCharacter.TimelessCharacter_C|GetQuestLogComponent (Variables|Default|GetAs%20Timeless%20Character)) self)
  (CallFunction|GenerateLoot)
  (Variables|Default|SetIsAlive? false))

(event Custom|Looted)

(event Custom|PlayDeathAnimation)

(event Custom|AnimalAttack)

(event Custom|AnimalAggroSound)

(event EventBeginPlay
  (bind _returnvalue (UserInterface|CreateWidget "/Game/Blueprints/UI/FloatingDamageTextContainer.FloatingDamageTextContainer_C"))
  (UserInterface|SetWidget (Variables|Default|GetFloatingDamageTextContainerWG) _returnvalue)
  (Variables|Default|SetHealth (Variables|Default|GetMaxHealth))
  (bind _astimeless_character (Utilities|Casting|CastToTimelessCharacter (Game|GetPlayerCharacter 0)))
  (Variables|Default|SetAs%20Timeless%20Character _astimeless_character))

(event EventInteract
  (params (Interactor :type Actor%20Object%20Reference))
  (if (Variables|Default|GetIsAlive?)
    (bind _asai_parent (Utilities|Casting|CastToAI_Parent (AI|GetAIController self)))
    (bind _output_get (Variables|Default|SetAs%20AI%20Parent _asai_parent))
    (AI|SetFocus _output_get Interactor)
    (AI|AIMoveTo _output_get "0, 0, 0" Interactor 2.5 "Default" "Default" true false
      (:then
        (switch int (Variables|/Game/Blueprints/NPCs/AI_Parent.AI_Parent_C|GetQuestNumber _output_get)
          (:0
            (AI|RunBehaviorTree (Variables|Default|GetAs%20AI%20Parent) (Variables|Default|GetBT1)))
          (:1
            (AI|RunBehaviorTree (Variables|Default|GetAs%20AI%20Parent) (Variables|Default|GetBT2))))))
    (else
      (Utilities|Casting|CastToTimelessCharacter Interactor)
      (Default|ToggleInventory (Variables|Default|GetInventoryComponent))
      (CallFunction|Looted))))

(event Game|Damage|EventAnyDamage
  (params (Damage :type Float%20%28single-precision%29) (DamageType :type Damage%20Type%20Object%20Reference) (InstigatedBy :type Controller%20Object%20Reference) (DamageCauser :type Actor%20Object%20Reference))
  (bind _self self)
  (bind _returnvalue (AI|GetAIController _self))
  (Variables|Default|SetHealth (- (Variables|Default|GetHealth) Damage))
  (bind _returnvalue_2 (UserInterface|CreateWidget "/Game/Blueprints/UI/FloatingDamageText.FloatingDamageText_C" 0 Damage))
  (Widget|Panel|AddChild (Variables|/Game/Blueprints/UI/FloatingDamageTextContainer.FloatingDamageTextContainer_C|GetDamageTextContainer (stale EventBeginPlay _returnvalue)) _returnvalue_2)
  (if (< (Variables|Default|GetHealth) 0.1)
    (bind _asai_hostile (Utilities|Casting|CastToAI_Hostile _returnvalue)
      (:then
        (Default|EventDie _asai_hostile))
      (:CastFailed
        (bind _asai_animals (Utilities|Casting|CastToAI_Animals _returnvalue))
        (Default|EventDie _asai_animals)))
    (Collision|SetCollisionEnabled (Variables|Collision|GetCapsuleComponent) "NoCollision")
    (Default|CheckKillObjective (Variables|/Game/Blueprints/TimelessCharacter.TimelessCharacter_C|GetQuestLogComponent (Variables|Default|GetAs%20Timeless%20Character)) self)
    (CallFunction|GenerateLoot)
    (Variables|Default|SetIsAlive? false)))

(fn ConstructionScript)

(fn RollLootTable
  (for _array_element (.lootstruct (Variables|Default|GetLootTable))
    (if (<= (Math|Random|RandomIntegerinRange 0 100) (.DropChance (Utilities|Struct|BreakLootStruct _array_element)))
      (Default|AddtoInventory (Variables|Default|GetInventoryComponent) (Utilities|Struct|MakeSlotStruct (.ItemStructure (Utilities|GetClassDefaults (.class (.itemstructure (.SlotStruct (Utilities|Struct|BreakLootStruct _array_element)))))) (.quantity (.SlotStruct (Utilities|Struct|BreakLootStruct _array_element)))) true))))