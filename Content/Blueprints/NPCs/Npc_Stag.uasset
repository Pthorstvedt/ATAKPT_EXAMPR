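; Stag NPC Blueprint that wanders the map and plays a death animation, extending a parent NPC class.
; On BeginPlay it sets a slow walk speed and moves to random navigable points around its current location, repeating after a brief delay only when a move succeeds.
; The death override calls the parent, then uses DoOnce to start a deer doe death montage on the mesh, set to loop.
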(event EventBeginPlay
  (bind _self self)
  (|CallParentFunction)
  (Variables|/Script/Engine.CharacterMovementComponent|SetMaxWalkSpeed (Variables|Character|GetCharacterMovement) 1.2e+02 :!label _label)
  (bind _randomlocation (Class|NavigationSystemV1|GetRandomLocationinNavigableRadius (Transformation|GetActorLocation _self) 4e+03 0 0))
  (AI|AIMoveTo _self _randomlocation 0 5.0 false
    (:OnSuccess
      (Utilities|FlowControl|Delay 0.1)
      (goto _label))))

(event EventPlayDeathAnimation
  (|CallParentFunction)
  (Utilities|FlowControl|DoOnce false
    (:Completed
      (Components|Animation|PlayAnimation (Variables|Character|GetMesh) "/Game/AnimalVarietyPack/DeerStagAndDoe/Animations/ANIM_DeerDoe_Death_Montage.ANIM_DeerDoe_Death_Montage" true))))

(fn ConstructionScript
  (|CallParentFunction))