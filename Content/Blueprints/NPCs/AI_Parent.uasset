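; AI_Parent is a base AI controller for NPCs, handling behavior tree startup, player focus and a quest counter.
; On possess it caches the ThirdPersonGameMode and runs the default behavior tree, which it runs again when a conversation ends.
; FocusOnPlayer focuses on the TimelessCharacter player and writes it to the FocusTarget blackboard key.
; Ending a conversation clears focus but leaves that key set, and a separate event increments the quest number.
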(event Custom|FocusOnPlayer
  (bind _astimeless_character (Utilities|Casting|CastToTimelessCharacter (Game|GetPlayerCharacter 0)))
  (AI|SetFocus _astimeless_character)
  (AI|Components|Blackboard|SetValueasObject (AI|GetBlackboard 0) (Utilities|Name|MakeLiteralName "FocusTarget") _astimeless_character))

(event Custom|ClearFocus
  (AI|ClearFocus))

(event Custom|IncrementQuestNumber
  (Variables|Default|SetQuestNumber (+ (Variables|Default|GetQuestNumber) 1)))

(event Custom|EndConversation
  (AI|ClearFocus)
  (AI|RunBehaviorTree (Variables|Default|GetDefaultBT)))

(event EventPossess
  (params (PossessedPawn :type Pawn%20Object%20Reference))
  (bind _asthird_person_game_mode (Utilities|Casting|CastToThirdPersonGameMode (Game|GetGameMode)))
  (Variables|Default|SetAs%20Third%20Person%20Game%20Mode _asthird_person_game_mode)
  (AI|RunBehaviorTree (Variables|Default|GetDefaultBT)))

(fn ConstructionScript)