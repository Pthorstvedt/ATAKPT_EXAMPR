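; AI controller for the spider enemy that runs its behavior tree on possession and drives combat music.
; Perception updates for TimelessCharacter set the CanSeeEnemy blackboard key and focus, toggling the combat state and switching music through ThirdPersonGameMode.
; Losing the target reverts the music after a short delay unless combat resumes.
; Death stops perception handling, updates the AI_State key and reuses that delayed combat exit.
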(event OnTargetPerceptionUpdated(AIPerception)
  (params (Actor :type Actor%20Object%20Reference) (Stimulus :type AI%20Stimulus%20Structure))
  (bind _as_third_person_game_mode (Variables|Default|GetAs%20Third%20Person%20Game%20Mode))
  (if (Variables|Default|GetIsAlive?)
    (bind _astimeless_character (Utilities|Casting|CastToTimelessCharacter Actor))
    (Variables|Default|SetCurrentTarget _astimeless_character)
    (AI|Components|Blackboard|SetValueasBool (AI|GetBlackboard 0) (Utilities|Name|MakeLiteralName "CanSeeEnemy") (.bsuccessfullysensed Stimulus))
    (if (.bsuccessfullysensed Stimulus)
      (AI|SetFocus _astimeless_character)
      (Variables|Default|SetCombat? true)
      (Default|ChangeMusic _as_third_person_game_mode "NewEnumerator1")
      (else
        (AI|ClearFocus)
        (Variables|Default|SetCombat? false)
        (Utilities|FlowControl|Delay 2.5)
        (if (not (Variables|Default|GetCombat?))
          (Default|ChangeMusic _as_third_person_game_mode "NewEnumerator0"))))))

(event Custom|Event%20Die
  (Variables|Default|SetIsAlive? false)
  (bind _output_get (Variables|Default|SetE_AI_State "NewEnumerator7"))
  (AI|Components|Blackboard|SetValueasEnum (AI|GetBlackboard 0) (Utilities|Name|MakeLiteralName "AI_State") _output_get)
  (AI|ClearFocus)
  (Variables|Default|SetCombat? false)
  (Utilities|FlowControl|Delay 2.5)
  (if (not (Variables|Default|GetCombat?))
    (Default|ChangeMusic (Variables|Default|GetAs%20Third%20Person%20Game%20Mode) "NewEnumerator0")))

(event EventPossess
  (params (PossessedPawn :type Pawn%20Object%20Reference))
  (AI|RunBehaviorTree "/Game/Blueprints/NPCs/Hostile/BT_EnemySpider.BT_EnemySpider")
  (bind _asthird_person_game_mode (Utilities|Casting|CastToThirdPersonGameMode (Game|GetGameMode)))
  (Variables|Default|SetAs%20Third%20Person%20Game%20Mode _asthird_person_game_mode))

(fn ConstructionScript)