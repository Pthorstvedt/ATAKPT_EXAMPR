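; AI controller for hostile humanoid NPCs that runs their behavior tree and reports combat to the game mode.
; Perception updates, while alive, store the sensed TimelessCharacter, write sight to the blackboard and set or clear focus.
; Sighting changes the music, while two mutually resetting DoOnce gates keep the combatant count from repeating increments or decrements.
; Die sets the AI state, clears focus and triggers the decrement gate.
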(event OnTargetPerceptionUpdated(AIPerception)
  (params (Actor :type Actor%20Object%20Reference) (Stimulus :type AI%20Stimulus%20Structure))
  (bind _as_third_person_game_mode_0 (Variables|Default|GetAs%20Third%20Person%20Game%20Mode_0))
  (if (Variables|Default|GetIsAlive?)
    (bind _astimeless_character (Utilities|Casting|CastToTimelessCharacter Actor))
    (Variables|Default|SetCurrentTarget _astimeless_character)
    (AI|Components|Blackboard|SetValueasBool (AI|GetBlackboard 0) (Utilities|Name|MakeLiteralName "CanSeeEnemy") (.bsuccessfullysensed Stimulus))
    (if (.bsuccessfullysensed Stimulus)
      (AI|SetFocus _astimeless_character)
      (Utilities|FlowControl|Sequence
        (:then_0
          (Default|ChangeMusic _as_third_person_game_mode_0 "NewEnumerator1")
          (Utilities|FlowControl|DoOnce false :!label _label
            (:Completed
              (Default|SetCombatants _as_third_person_game_mode_0 1))))
        (:then_1
          (goto _label_2 Reset)))
      (else
        (AI|ClearFocus)
        (Utilities|FlowControl|Sequence
          (:then_0
            (goto _label Reset))
          (:then_1
            (Utilities|FlowControl|DoOnce false :!label _label_2
              (:Completed
                (Default|SetCombatants _as_third_person_game_mode_0 -1)))))))))

(event Custom|Event%20Die
  (Variables|Default|SetIsAlive? false)
  (bind _output_get (Variables|Default|SetE_AI_State "NewEnumerator7"))
  (AI|Components|Blackboard|SetValueasEnum (AI|GetBlackboard 0) (Utilities|Name|MakeLiteralName "AI_State") _output_get)
  (AI|ClearFocus)
  (Utilities|FlowControl|DoOnce false
    (:Completed
      (Default|SetCombatants (Variables|Default|GetAs%20Third%20Person%20Game%20Mode_0) -1))))

(event EventTick
  (params (DeltaSeconds :type Float%20%28single-precision%29)))

(event EventPossess
  (params (PossessedPawn :type Pawn%20Object%20Reference))
  (bind _asthird_person_game_mode (Utilities|Casting|CastToThirdPersonGameMode (Game|GetGameMode)))
  (Variables|Default|SetAs%20Third%20Person%20Game%20Mode_0 _asthird_person_game_mode)
  (AI|RunBehaviorTree "/Game/Blueprints/NPCs/Hostile/BT_EnemyHumanoid.BT_EnemyHumanoid"))

(fn ConstructionScript
  (|CallParentFunction))