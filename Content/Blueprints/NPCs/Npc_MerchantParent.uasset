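; Parent Blueprint for merchant NPCs that fills its inventory component from a loot inventory when an actor overlaps it.
; Each loot entry is written to the same inventory index, taking item data from the item class defaults and keeping the entry's quantity.
; The copy reruns on every overlap without filtering the actor, and prints a debug "Hello" per entry.
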(event EventBeginPlay
  (|CallParentFunction))

(event Collision|EventActorBeginOverlap
  (params (OtherActor :type Actor%20Object%20Reference))
  (|CallParentFunction OtherActor)
  (for (_array_element _array_index) (.inventory (Variables|Default|GetLootInventory))
    (Utilities|Array|SetArrayElem (Variables|/Game/Blueprints/Inventory/InventoryComponent.InventoryComponent_C|GetInventory (Variables|Default|GetInventoryComponent)) _array_index (Utilities|Struct|MakeSlotStruct (.ItemStructure (Utilities|GetClassDefaults (.class (.ItemStructure (Utilities|Struct|BreakSlotStruct _array_element))))) (.Quantity (Utilities|Struct|BreakSlotStruct _array_element))))
    (Development|PrintString "Hello")))

(event EventTick
  (params (DeltaSeconds :type Float%20%28single-precision%29))
  (|CallParentFunction DeltaSeconds) ; This node is disabled and will not be called.\nDrag off pins to build functionality.
)

(fn ConstructionScript
  (|CallParentFunction))