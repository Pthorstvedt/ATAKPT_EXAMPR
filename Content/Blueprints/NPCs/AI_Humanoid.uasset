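; AI controller for humanoid NPCs that runs the BT_EnemyHumanoid behavior tree on possession and again when a conversation ends.
; Perception updates on the player character set focus and the CanSeeEnemy blackboard key, and sightings trigger a music change through the game mode.
; Paired DoOnce gates add or remove one combatant in the game mode as sight is gained or lost.
; Death updates the AI_State key, clears focus and releases the combatant count.
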(event OnTargetPerceptionUpdated(AIPerception)
  (params (Actor :type Actor%20Object%20Reference) (Stimulus :type AI%20Stimulus%20Structure))
  (bind _as_third_person_game_mode (Variables|Default|GetAs%20Third%20Person%20Game%20Mode))
  (if (Variables|Default|GetIsAlive?)
    (bind _astimeless_character (Utilities|Casting|CastToTimelessCharacter Actor))
    (Variables|Default|SetCurrentTarget _astimeless_character)
    (AI|Components|Blackboard|SetValueasBool (AI|GetBlackboard 0) (Utilities|Name|MakeLiteralName "CanSeeEnemy") (.bsuccessfullysensed Stimulus))
    (if (.bsuccessfullysensed Stimulus)
      (AI|SetFocus _astimeless_character)
      (Utilities|FlowControl|Sequence
        (:then_0
          (Default|ChangeMusic _as_third_person_game_mode "NewEnumerator1")
          (Utilities|FlowControl|DoOnce false :!label _label
            (:Completed
              (Default|SetCombatants _as_third_person_game_mode 1))))
        (:then_1
          (goto _label_2 Reset)))
      (else
        (AI|ClearFocus)
        (Utilities|FlowControl|Sequence
          (:then_0
            (goto _label Reset))
          (:then_1
            (Utilities|FlowControl|DoOnce false :!label _label_2
              (:Completed
                (Default|SetCombatants _as_third_person_game_mode -1)))))))))

(event Custom|Event%20Die
  (Variables|Default|SetIsAlive? false)
  (bind _output_get (Variables|Default|SetE_AI_State "NewEnumerator7"))
  (AI|Components|Blackboard|SetValueasEnum (AI|GetBlackboard 0) (Utilities|Name|MakeLiteralName "AI_State") _output_get)
  (AI|ClearFocus)
  (Utilities|FlowControl|DoOnce false
    (:Completed
      (Default|SetCombatants (Variables|Default|GetAs%20Third%20Person%20Game%20Mode) -1))))

(event Custom|EndConversation
  (AI|RunBehaviorTree "/Game/Blueprints/NPCs/Hostile/BT_EnemyHumanoid.BT_EnemyHumanoid"))

(event Custom|IncrementQuestNumber
  (Variables|Default|SetQuestNumber (+ (Variables|Default|GetQuestNumber) 1)))

(event EventPossess
  (params (PossessedPawn :type Pawn%20Object%20Reference))
  (AI|RunBehaviorTree "/Game/Blueprints/NPCs/Hostile/BT_EnemyHumanoid.BT_EnemyHumanoid")
  (bind _asthird_person_game_mode (Utilities|Casting|CastToThirdPersonGameMode (Game|GetGameMode)))
  (Variables|Default|SetAs%20Third%20Person%20Game%20Mode _asthird_person_game_mode))

(fn ConstructionScript)