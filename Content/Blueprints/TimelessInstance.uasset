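; TimelessInstance is the game instance that holds and saves player progress.
; On Init or OpenLevel it sets focus to the game viewport, then loads the save object from its named slot or creates a new one.
; SavePlayerData copies transform, inventory, attributes, equipment, quests, objective progress and silver into that object and writes it to the slot.
; The SaveGame function only caches the player's TimelessCharacter, without saving anything.
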(event Custom|SavePlayerData
  (params (PlayerPosition :type Transform) (Inventory :type Array%20of%20Slot%20Struct%20Structures) (Attributes :type Attribute%20Struct%20Structure) (EquippedItems :type Map%20of%20E_SlotType%20Enums%20to%20Structs :default "NewEnumerator0") (Quests :type Array%20of%20Q%200%20Quest%20Parent%20Object%20References) (QuestProgress :type Map%20of%20Strings%20to%20Booleans) (Silver :type Integer))
  (bind _savegamedata (Variables|Default|GetSaveGameData))
  (bind _savegamename (Variables|Default|GetSaveGameName))
  (Variables|/Game/Blueprints/SaveGameObject.SaveGameObject_C|SetPlayerTransform_Save _savegamedata PlayerPosition)
  (Variables|/Game/Blueprints/SaveGameObject.SaveGameObject_C|SetPlayerInventory_Save _savegamedata Inventory)
  (Variables|/Game/Blueprints/SaveGameObject.SaveGameObject_C|SetPlayerAttributes_Save _savegamedata Attributes)
  (Variables|/Game/Blueprints/SaveGameObject.SaveGameObject_C|SetPlayerEquipped_Save _savegamedata EquippedItems)
  (Variables|/Game/Blueprints/SaveGameObject.SaveGameObject_C|SetPlayerQuests_Save _savegamedata Quests)
  (Variables|/Game/Blueprints/SaveGameObject.SaveGameObject_C|SetQuestObjectiveProgress_Save _savegamedata QuestProgress)
  (Variables|/Game/Blueprints/SaveGameObject.SaveGameObject_C|SetCurrencySilver_Save _savegamedata Silver)
  (SaveGame|SaveGametoSlot _savegamedata _savegamename)
  (Development|PrintString _savegamename))

(event Custom|OpenLevel
  (Class|WidgetBlueprintLibrary|SetFocustoGameViewport)
  (bind _returnvalue (SaveGame|DoesSaveGameExist (Variables|Default|GetSaveGameName)))
  (if _returnvalue
    (bind _returnvalue_2 (SaveGame|LoadGamefromSlot (Variables|Default|GetSaveGameName)))
    (bind _assave_game_object (Utilities|Casting|CastToSaveGameObject _returnvalue_2))
    (Variables|Default|SetSaveGameData _assave_game_object)
    (else
      (bind _returnvalue_3 (SaveGame|CreateSaveGameObject "/Game/Blueprints/SaveGameObject.SaveGameObject_C"))
      (Variables|Default|SetSaveGameData _returnvalue_3))))

(event EventInit
  (Class|WidgetBlueprintLibrary|SetFocustoGameViewport)
  (bind _returnvalue (SaveGame|DoesSaveGameExist (Variables|Default|GetSaveGameName)))
  (if _returnvalue
    (bind _returnvalue_2 (SaveGame|LoadGamefromSlot (Variables|Default|GetSaveGameName)))
    (bind _assave_game_object (Utilities|Casting|CastToSaveGameObject _returnvalue_2))
    (Variables|Default|SetSaveGameData _assave_game_object)
    (else
      (bind _returnvalue_3 (SaveGame|CreateSaveGameObject "/Game/Blueprints/SaveGameObject.SaveGameObject_C"))
      (Variables|Default|SetSaveGameData _returnvalue_3))))

(fn SaveGame
  (bind _astimeless_character (Utilities|Casting|CastToTimelessCharacter (Game|GetPlayerCharacter 0)))
  (LocalVariables|SetPlayerCharacter _astimeless_character))