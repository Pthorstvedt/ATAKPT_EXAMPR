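; Test target dummy that takes damage and shows it as floating damage text.
; BeginPlay places a text container widget in its widget component, and each AnyDamage event lowers Health and adds a new damage text to that container.
; Overlaps on the head, chest and two arm colliders set a body-part damage modifier, which this Blueprint's damage handling does not apply.
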(event OnComponentBeginOverlap(ChestCollision)
  (params (OverlappedComponent :type Primitive%20Component%20Object%20Reference) (OtherActor :type Actor%20Object%20Reference) (OtherComp :type Primitive%20Component%20Object%20Reference) (OtherBodyIndex :type Integer) (bFromSweep :type Boolean) (SweepResult :type Hit%20Result%20Structure%20%28by%20ref%29))
  (Variables|Default|SetBodyPartDMGmod 1.0))

(event OnComponentBeginOverlap(HeadCollision)
  (params (OverlappedComponent :type Primitive%20Component%20Object%20Reference) (OtherActor :type Actor%20Object%20Reference) (OtherComp :type Primitive%20Component%20Object%20Reference) (OtherBodyIndex :type Integer) (bFromSweep :type Boolean) (SweepResult :type Hit%20Result%20Structure%20%28by%20ref%29))
  (Variables|Default|SetBodyPartDMGmod 2.0))

(event OnComponentBeginOverlap(ArmCollision)
  (params (OverlappedComponent :type Primitive%20Component%20Object%20Reference) (OtherActor :type Actor%20Object%20Reference) (OtherComp :type Primitive%20Component%20Object%20Reference) (OtherBodyIndex :type Integer) (bFromSweep :type Boolean) (SweepResult :type Hit%20Result%20Structure%20%28by%20ref%29))
  (Variables|Default|SetBodyPartDMGmod 0.5))

(event OnComponentBeginOverlap(Armcollision2)
  (params (OverlappedComponent :type Primitive%20Component%20Object%20Reference) (OtherActor :type Actor%20Object%20Reference) (OtherComp :type Primitive%20Component%20Object%20Reference) (OtherBodyIndex :type Integer) (bFromSweep :type Boolean) (SweepResult :type Hit%20Result%20Structure%20%28by%20ref%29))
  (Variables|Default|SetBodyPartDMGmod 0.5))

(event EventBeginPlay
  (bind _returnvalue (UserInterface|CreateWidget "/Game/Blueprints/UI/FloatingDamageTextContainer.FloatingDamageTextContainer_C"))
  (UserInterface|SetWidget (Variables|Default|GetDamageContainerWidget) _returnvalue))

(event Game|Damage|EventAnyDamage
  (params (Damage :type Float%20%28single-precision%29) (DamageType :type Damage%20Type%20Object%20Reference) (InstigatedBy :type Controller%20Object%20Reference) (DamageCauser :type Actor%20Object%20Reference))
  (Variables|Default|SetHealth (- (Variables|Default|GetHealth) Damage))
  (bind _returnvalue (UserInterface|CreateWidget "/Game/Blueprints/UI/FloatingDamageText.FloatingDamageText_C" 0 Damage))
  (Widget|Panel|AddChild (Variables|/Game/Blueprints/UI/FloatingDamageTextContainer.FloatingDamageTextContainer_C|GetDamageTextContainer (stale EventBeginPlay _returnvalue)) _returnvalue))

(fn ConstructionScript)