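; Quest log component that holds the player's quests and completes their location, collection and delivery objectives.
; Check functions match objective targets, query the player's inventory for item objectives (removing items on delivery), then flag the objective and re-evaluate quest completion.
; Progress lives in a map keyed by quest name plus objective description, seeded from the GameInstance save data and reapplied to quests shortly after BeginPlay.
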(event Custom|AddQuest
  (params (QuestToAdd :type Quest%20Parent%20Object%20Reference))
  (bind _quests (Variables|Default|GetQuests))
  (if (Utilities|Array|ContainsItem _quests QuestToAdd)
    (Development|PrintString "QuestLogComponent: Already have this Quest!" true true "(R=1.000000,G=0.049283,B=0.960843,A=1.000000)" 5.0)
    (else
      (Utilities|Array|Add _quests QuestToAdd)
      (for _array_element (Variables|/Game/Blueprints/QuestLog/Quests/Quest_Parent.Quest_Parent_C|GetObjectives QuestToAdd)
        (Utilities|Map|Add (Variables|Default|GetQuestObjectiveProgress) (Utilities|String|ToString(Text) (Utilities|Text|FormatText "{Questname}+{Objectivedesc}" (Variables|/Game/Blueprints/QuestLog/Quests/Quest_Parent.Quest_Parent_C|GetQuestName QuestToAdd) (.ObjectiveDescription (Utilities|Struct|BreakObjectiveStruct _array_element)))) (.IsComplete? (Utilities|Struct|BreakObjectiveStruct _array_element)))))))

(event EventBeginPlay
  (bind _astimeless_character (Utilities|Casting|CastToTimelessCharacter (Game|GetPlayerCharacter 0)))
  (Variables|Default|SetAs%20Timeless%20Character _astimeless_character)
  (bind _astimeless_instance (Utilities|Casting|CastToTimelessInstance (Game|GetGameInstance)))
  (bind _output_get (Variables|Default|SetAs%20Timeless%20Instance _astimeless_instance))
  (Variables|Default|SetQuestObjectiveProgress (Variables|/Game/Blueprints/SaveGameObject.SaveGameObject_C|GetQuestObjectiveProgress_Save (Variables|/Game/Blueprints/TimelessInstance.TimelessInstance_C|GetSaveGameData _output_get)))
  (Utilities|FlowControl|Delay 0.2)
  (CallFunction|LoadObjectiveProgress))

(fn CheckLocationObjective
  (params (LocationTrigger :type Actor%20Object%20Reference))
  (for (_array_element _array_index) (Variables|Default|GetQuests)
    (Utilities|IsValid _array_element
      (:Is%20Valid
        (LocalVariables|SetQuestChecked _array_element)
        (LocalVariables|SetQuestIndex _array_index)
        (if (not (Variables|/Game/Blueprints/QuestLog/Quests/Quest_Parent.Quest_Parent_C|GetQuestComplete? _array_element))
          (bind (_array_element_2 _array_index_2) (Utilities|Array|ForEachLoopwithBreak (Variables|/Game/Blueprints/QuestLog/Quests/Quest_Parent.Quest_Parent_C|GetObjectives _array_element) :!label _label)
            (:LoopBody
              (bind _output_get (LocalVariables|SetObjectiveChecked _array_element_2))
              (if (and (Utilities|Enum|Equal(Enum) (.objectivetype _output_get) "NewEnumerator0") (not (.iscomplete? _output_get)))
                (if (== (.target _output_get) LocationTrigger)
                  (Utilities|Array|SetArrayElem (Variables|/Game/Blueprints/QuestLog/Quests/Quest_Parent.Quest_Parent_C|GetObjectives _array_element) _array_index_2 (Utilities|Struct|MakeObjectiveStruct (.objectivedescription (LocalVariables|GetObjectiveChecked)) (.objectivetype (LocalVariables|GetObjectiveChecked)) (.number (LocalVariables|GetObjectiveChecked)) true (.target (LocalVariables|GetObjectiveChecked)) (.objectiveimage (LocalVariables|GetObjectiveChecked))))
                  (bind _output_get_2 (LocalVariables|SetObjectiveFound? true))
                  (Utilities|Map|Add (Variables|Default|GetQuestObjectiveProgress) (Utilities|String|ToString(Text) (Utilities|Text|FormatText "{Questname}+{Objectivedesc}" (Variables|/Game/Blueprints/QuestLog/Quests/Quest_Parent.Quest_Parent_C|GetQuestName (LocalVariables|GetQuestChecked)) (.objectivedescription (LocalVariables|GetObjectiveChecked)))) _output_get_2)
                  (Default|CallObjectiveComplete)
                  (CallFunction|CheckQuestComplete (LocalVariables|GetQuestChecked))
                  (goto _label Break)))))))))
  (return (LocalVariables|GetObjectiveFound?)))

(fn CheckQuestComplete
  (params (QuestToCheck :type Quest%20Parent%20Object%20Reference))
  (for _array_element (Variables|/Game/Blueprints/QuestLog/Quests/Quest_Parent.Quest_Parent_C|GetObjectives QuestToCheck)
    (if (not (.iscomplete? _array_element))
      (return false)))
  (bind _output_get (Variables|/Game/Blueprints/QuestLog/Quests/Quest_Parent.Quest_Parent_C|SetQuestComplete? QuestToCheck true))
  (return _output_get))

(fn CheckCollectionObjective
  (params (ItemCollected :type Item%20Struct%20Structure))
  (for _array_element (Variables|Default|GetQuests)
    (Utilities|IsValid _array_element
      (:Is%20Valid
        (LocalVariables|SetCheckedQuest _array_element)
        ;[1 1 1] Skips Complete Quests
        (if (not (Variables|/Game/Blueprints/QuestLog/Quests/Quest_Parent.Quest_Parent_C|GetQuestComplete? _array_element))
          (for (_array_element_2 _array_index) (Variables|/Game/Blueprints/QuestLog/Quests/Quest_Parent.Quest_Parent_C|GetObjectives _array_element)
            (bind _output_get (LocalVariables|SetCheckedObjective _array_element_2))
            ;[1 1 1] Only checks Collect Objectives
            (LocalVariables|SetCheckedIndex _array_index)
            (if (Utilities|Enum|Equal(Enum) (.objectivetype _output_get) "NewEnumerator2")
              (if (== (Utilities|GetClass (.target _output_get)) (.class ItemCollected))
                (bind (_hasitems_ _amountofqueryitems) (Default|InventoryQuery (Variables|/Game/Blueprints/TimelessCharacter.TimelessCharacter_C|GetInventoryComponent (Variables|Default|GetAs%20Timeless%20Character)) (.class ItemCollected) (.number (LocalVariables|GetCheckedObjective))))
                (Utilities|FlowControl|Sequence
                  (:then_0
                    (if _hasitems_
                      (Utilities|Array|SetArrayElem (Variables|/Game/Blueprints/QuestLog/Quests/Quest_Parent.Quest_Parent_C|GetObjectives _array_element) (LocalVariables|GetCheckedIndex) (Utilities|Struct|MakeObjectiveStruct (.objectivedescription (LocalVariables|GetCheckedObjective)) (.objectivetype (LocalVariables|GetCheckedObjective)) (.number (LocalVariables|GetCheckedObjective)) true (.target (LocalVariables|GetCheckedObjective)) (.objectiveimage (LocalVariables|GetCheckedObjective))))
                      (Utilities|Map|Add (Variables|Default|GetQuestObjectiveProgress) (Utilities|String|ToString(Text) (Utilities|Text|FormatText "{Questname}+{Objectivedesc}" (Variables|/Game/Blueprints/QuestLog/Quests/Quest_Parent.Quest_Parent_C|GetQuestName (LocalVariables|GetCheckedQuest)) (.objectivedescription (LocalVariables|GetCheckedObjective)))) true)
                      (Default|CallObjectiveComplete)
                      (CallFunction|CheckQuestComplete (LocalVariables|GetCheckedQuest))))
                  (:then_1
                    (Development|PrintString (Utilities|String|ToString(Text) (Utilities|Text|FormatText "You have {NumberOfItems}/{QueryNumber} {Items}" _amountofqueryitems (.number (LocalVariables|GetCheckedObjective)) (.name ItemCollected))))))))))))))

(fn LoadObjectiveProgress
  (for _array_element (Variables|Default|GetQuests)
    (Utilities|IsValid _array_element
      (:Is%20Valid
        (LocalVariables|SetQuestChecked _array_element)
        (for (_array_element_2 _array_index) (Variables|/Game/Blueprints/QuestLog/Quests/Quest_Parent.Quest_Parent_C|GetObjectives _array_element)
          (bind _output_get (LocalVariables|SetObjectiveChecked _array_element_2))
          (if (.ReturnValue (Utilities|Map|Find (Variables|Default|GetQuestObjectiveProgress) (Utilities|String|ToString(Text) (Utilities|Text|FormatText "{Questname}+{Objectivedesc}" (Variables|/Game/Blueprints/QuestLog/Quests/Quest_Parent.Quest_Parent_C|GetQuestName (LocalVariables|GetQuestChecked)) (.objectivedescription _output_get)))))
            (Utilities|Array|SetArrayElem (Variables|/Game/Blueprints/QuestLog/Quests/Quest_Parent.Quest_Parent_C|GetObjectives _array_element) _array_index (Utilities|Struct|MakeObjectiveStruct (.objectivedescription (LocalVariables|GetObjectiveChecked)) (.objectivetype (LocalVariables|GetObjectiveChecked)) (.number (LocalVariables|GetObjectiveChecked)) (.Value (Utilities|Map|Find (Variables|Default|GetQuestObjectiveProgress) (Utilities|String|ToString(Text) (Utilities|Text|FormatText "{Questname}+{Objectivedesc}" (Variables|/Game/Blueprints/QuestLog/Quests/Quest_Parent.Quest_Parent_C|GetQuestName (LocalVariables|GetQuestChecked)) (.objectivedescription _output_get))))) (.target (LocalVariables|GetObjectiveChecked)) (.objectiveimage (LocalVariables|GetObjectiveChecked))))
            (else
              (Development|PrintString "LoadObjectiveProgress:Can't Find Objective" true true "(R=1.000000,G=0.421051,B=0.000000,A=1.000000)" 5.0))))
        (CallFunction|CheckQuestComplete (LocalVariables|GetQuestChecked))))))

(fn CheckDeliverObjective
  (params (StashActor :type Actor%20Object%20Reference) (ItemToDeliver :type Item%20Struct%20Structure))
  (bind _as_timeless_character (Variables|Default|GetAs%20Timeless%20Character))
  (bind _inventorycomponent (Variables|/Game/Blueprints/TimelessCharacter.TimelessCharacter_C|GetInventoryComponent _as_timeless_character))
  (for _array_element (Variables|Default|GetQuests)
    (Utilities|IsValid _array_element
      (:Is%20Valid
        (LocalVariables|SetQuestChecked _array_element)
        (if (not (Variables|/Game/Blueprints/QuestLog/Quests/Quest_Parent.Quest_Parent_C|GetQuestComplete? _array_element))
          (bind (_array_element_2 _array_index) (Utilities|Array|ForEachLoopwithBreak (Variables|/Game/Blueprints/QuestLog/Quests/Quest_Parent.Quest_Parent_C|GetObjectives _array_element) :!label _label)
            (:LoopBody
              (bind _output_get (LocalVariables|SetObjectiveChecked _array_element_2))
              (if (and (Utilities|Enum|Equal(Enum) (.objectivetype _output_get) "NewEnumerator1") (not (.iscomplete? _output_get)))
                (if (== (.target _output_get) StashActor)
                  (bind _hasitems_ (Default|InventoryQuery _inventorycomponent (.class ItemToDeliver) (.number (LocalVariables|GetObjectiveChecked))))
                  (if _hasitems_
                    (Default|RemovefromInventory _inventorycomponent ItemToDeliver (.number (LocalVariables|GetObjectiveChecked)))
                    (Utilities|Array|SetArrayElem (Variables|/Game/Blueprints/QuestLog/Quests/Quest_Parent.Quest_Parent_C|GetObjectives _array_element) _array_index (Utilities|Struct|MakeObjectiveStruct (.objectivedescription (LocalVariables|GetObjectiveChecked)) (.objectivetype (LocalVariables|GetObjectiveChecked)) (.number (LocalVariables|GetObjectiveChecked)) true (.target (LocalVariables|GetObjectiveChecked)) (.objectiveimage (LocalVariables|GetObjectiveChecked))))
                    (bind _output_get_2 (LocalVariables|SetObjectiveFound? true))
                    (Utilities|Map|Add (Variables|Default|GetQuestObjectiveProgress) (Utilities|String|ToString(Text) (Utilities|Text|FormatText "{Questname}+{Objectivedesc}" (Variables|/Game/Blueprints/QuestLog/Quests/Quest_Parent.Quest_Parent_C|GetQuestName (LocalVariables|GetQuestChecked)) (.objectivedescription (LocalVariables|GetObjectiveChecked)))) _output_get_2)
                    (Default|CallObjectiveComplete)
                    (CallFunction|CheckQuestComplete (LocalVariables|GetQuestChecked))
                    (goto _label Break))))))))))
  (return (LocalVariables|GetObjectiveFound?)))